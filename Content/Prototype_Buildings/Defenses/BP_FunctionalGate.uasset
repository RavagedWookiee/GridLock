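; Defensive gate Blueprint whose two doors swing open while anything overlaps its PipOpen trigger.
; A Pips counter rises on each overlap begin and opens the gate, then falls on overlap end and closes it at zero or below.
; Open and Close snap both doors to fixed world-space rotations with no animation, independent of the actor's own rotation.
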(event `self.PipOpen.OnComponentBeginOverlap`
  (params (OverlappedComponent :type "PrimitiveComponent Object Reference") (OtherActor :type "Actor Object Reference") (OtherComp :type "PrimitiveComponent Object Reference") (OtherBodyIndex :type Integer) (bFromSweep :type Boolean) (SweepResult :type "HitResult Structure (by ref)"))
  (set `self.Pips` (+ (`self.Pips`) 1))
  (`self.Open`))

(event `self.PipOpen.OnComponentEndOverlap`
  (params (OverlappedComponent :type "PrimitiveComponent Object Reference") (OtherActor :type "Actor Object Reference") (OtherComp :type "PrimitiveComponent Object Reference") (OtherBodyIndex :type Integer))
  (bind _output_get (set `self.Pips` (- (`self.Pips`) 1)))
  (`/Engine/EditorBlueprintResources/StandardMacros.CompareInt` _output_get
    (:`==`
      _)
    (:`<`
      _))
  (`self.Close`))

(fn `Close`
  (`SceneComponent.K2_SetWorldRotation` :`self` (`self.RightDoor`))
  (`SceneComponent.K2_SetWorldRotation` :`self` (`self.LeftDoor`)))

(fn `Open`
  (`SceneComponent.K2_SetWorldRotation` (`self.RightDoor`) (struct :`Yaw` -90.0) false false)
  (`SceneComponent.K2_SetWorldRotation` (`self.LeftDoor`) (struct :`Yaw` 90.0) false false))

(fn `UserConstructionScript`)